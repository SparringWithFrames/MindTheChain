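; Cable node that tethers the player, tracks power across visited nodes and hosts either a portal or gravity well.
; Entering range attaches the cuff, enables input and adjusts power, shown by cable colour; linked nodes reroute the grid cable.
; At full power, mouse clicks place either device; active portals teleport player and blocks, while wells lift blocks or roll the world via timeline.
; A shared Transit flag with delays serves as cooldown.
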(event OnComponentBeginOverlap(GravityWell)
  (params (OverlappedComponent :type Primitive%20Component%20Object%20Reference) (OtherActor :type Actor%20Object%20Reference) (OtherComp :type Primitive%20Component%20Object%20Reference) (OtherBodyIndex :type Integer) (bFromSweep :type Boolean) (SweepResult :type Hit%20Result%20Structure%20%28by%20ref%29))
  (bind _pcharacter (Variables|Default|GetPcharacter))
  ;[1 1 1] Block Enters Gravity Well
  (bind _returnvalue (Class|MindtheChainCharacter|GetTransit (Variables|Default|GetPcharacter)))
  (if (not _returnvalue)
    (if (Variables|Default|GetWellActive)
      (bind _asmod_block (Utilities|Casting|CastToMod_Block OtherActor))
      (Physics|SetSimulatePhysics (Variables|/Script/Engine.StaticMeshActor|GetStaticMeshComponent _asmod_block) false)
      (Physics|SetSimulatePhysics (Variables|/Script/Engine.StaticMeshActor|GetStaticMeshComponent _asmod_block) true)
      (Physics|SetPhysicsLinearVelocity (Variables|/Script/Engine.StaticMeshActor|GetStaticMeshComponent _asmod_block) "0, 0,9.800000" false "None")
      (Class|MindtheChainCharacter|SetTransit _pcharacter true)
      (Utilities|FlowControl|Delay 5.0)
      (Class|MindtheChainCharacter|SetTransit _pcharacter false))))

(event OnActorBeginOverlap(CableCon)
  (params (OverlappedActor :type Actor%20Object%20Reference) (OtherActor :type Actor%20Object%20Reference))
  (bind _cablecon (Variables|Default|GetCableCon))
  ;[1 1 1] Check Visited
  (Utilities|Casting|CastToMindTheChainCharacter OtherActor)
  (Class|CableComponent|SetAttachEndtoComponent (Variables|Default|GetGrid) (Variables|BP_Cable_C|GetSphere _cablecon) "None")
  (if (Variables|BP_Cable_C|GetVisited _cablecon)
    (Rendering|SetVisibility (Variables|Default|GetGrid) false false)
    (Variables|Default|SetVisited false)))

(event OnActorBeginOverlap(CableConGrav)
  (params (OverlappedActor :type Actor%20Object%20Reference) (OtherActor :type Actor%20Object%20Reference))
  (bind _cablecongrav (Variables|Default|GetCableConGrav))
  ;[1 1 1] Check Visited
  (Utilities|Casting|CastToMindTheChainCharacter OtherActor)
  (Class|CableComponent|SetAttachEndtoComponent (Variables|Default|GetGrid) (Variables|BP_Cable_C|GetSphere _cablecongrav) "None")
  (if (Variables|BP_Cable_C|GetVisited _cablecongrav)
    (Rendering|SetVisibility (Variables|Default|GetGrid) false false)
    (Variables|Default|SetVisited false)))

(event OnComponentBeginOverlap(PortalRange)
  (params (OverlappedComponent :type Primitive%20Component%20Object%20Reference) (OtherActor :type Actor%20Object%20Reference) (OtherComp :type Primitive%20Component%20Object%20Reference) (OtherBodyIndex :type Integer) (bFromSweep :type Boolean) (SweepResult :type Hit%20Result%20Structure%20%28by%20ref%29))
  (bind _portal_range (Variables|Default|GetPortal%20Range))
  (bind _pcharacter (Variables|Default|GetPcharacter))
  (bind _pcharacter_2 (Variables|Default|GetPcharacter))
  (bind _returnvalue (Physics|GetCenterOfMass _portal_range "None"))
  ;[1 1 1] Block Teleport
  (bind _returnvalue_2 (Class|MindtheChainCharacter|GetTransit (Variables|Default|GetPcharacter)))
  (if (not _returnvalue_2)
    (bind _asmod_block (Utilities|Casting|CastToMod_Block OtherActor))
    (if (and (not (Variables|/Game/Blueprints/Mod_Block.Mod_Block_C|GetRecentlyPorted _asmod_block)) (Variables|Default|GetPortalActive))
      (bind _returnvalue_3 (Class|MindtheChainCharacter|GetPortalCoordinates _pcharacter_2 _returnvalue))
      (if (not (Math|Vector|Equal(Vector) _returnvalue_3 "0, 0, 0" 0.0001))
        (Variables|/Game/Blueprints/Mod_Block.Mod_Block_C|SetRecentlyPorted _asmod_block true)
        (bind _returnvalue_4 (Class|MindtheChainCharacter|GetVol _pcharacter_2))
        (Audio|PlaySoundatLocation "/Game/Audio/482231__veromarengere__02-lasers.482231__veromarengere__02-lasers" _returnvalue "0, 0, 0" (* _returnvalue_4 1.0) 1.0 0.0 "/Game/Audio/NewSoundAttenuation.NewSoundAttenuation" 0 0)
        (Transformation|Teleport _asmod_block _returnvalue_3 "0, 0, 0")
        ;[1 1 1] Hack -> Component your teleporting to begins its overlap function before this fires
        (Variables|/Game/Blueprints/Mod_Block.Mod_Block_C|SetRecentlyPorted _asmod_block false)
        (Physics|SetSimulatePhysics (Variables|/Script/Engine.StaticMeshActor|GetStaticMeshComponent _asmod_block) false)
        (Physics|SetSimulatePhysics (Variables|/Script/Engine.StaticMeshActor|GetStaticMeshComponent _asmod_block) true)
        (Physics|SetEnableGravity (Variables|/Script/Engine.StaticMeshActor|GetStaticMeshComponent _asmod_block) true)
        (Class|MindtheChainCharacter|SetTransit _pcharacter true)
        (Utilities|FlowControl|Delay 3.0)
        (Class|MindtheChainCharacter|SetTransit _pcharacter false)
        (Physics|SetSimulatePhysics (Variables|/Script/Engine.StaticMeshActor|GetStaticMeshComponent _asmod_block) false)
        (Physics|SetEnableGravity (Variables|/Script/Engine.StaticMeshActor|GetStaticMeshComponent _asmod_block) false)))))

(event OnComponentBeginOverlap(CableRange)
  (params (OverlappedComponent :type Primitive%20Component%20Object%20Reference) (OtherActor :type Actor%20Object%20Reference) (OtherComp :type Primitive%20Component%20Object%20Reference) (OtherBodyIndex :type Integer) (bFromSweep :type Boolean) (SweepResult :type Hit%20Result%20Structure%20%28by%20ref%29))
  (bind _returnvalue (Game|GetPlayerCharacter 0))
  (bind _pcharacter (Variables|Default|GetPcharacter))
  (bind _cuff (Variables|Default|GetCuff))
  ;[1 1 1] Visiting
  (Utilities|Casting|CastToCapsuleComponent OtherComp)
  (Utilities|Set|Tether _pcharacter (Transformation|GetActorLocation _pcharacter))
  (if (or (Variables|Default|GetPortalActive) (Variables|Default|GetWellActive))
    _
    (elif (Variables|Default|GetVisited)
      (bind _asfirst_person_character (Utilities|Casting|CastToFirstPersonCharacter _pcharacter))
      (if (Variables|/Game/FirstPersonCPP/Blueprints/FirstPersonCharacter.FirstPersonCharacter_C|Getrecentlyactivated _asfirst_person_character)
        (Variables|/Game/FirstPersonCPP/Blueprints/FirstPersonCharacter.FirstPersonCharacter_C|Setrecentlyactivated _asfirst_person_character false)
        (else
          (Class|MindtheChainCharacter|RemovePower _pcharacter)
          (CallFunction|UpdateCableMats)))
      (else
        (Class|MindtheChainCharacter|AddPower _pcharacter)
        (CallFunction|UpdateCableMats))))
  (Rendering|SetVisibility _cuff true false)
  (Class|CableComponent|SetAttachEndto _cuff _returnvalue "None" "None")
  (bind _returnvalue_2 (Class|MindtheChainCharacter|GetRecentlyPorted (Variables|Default|GetPcharacter)))
  (if (not _returnvalue_2)
    (Rendering|SetVisibility (Variables|Default|GetGrid) true false)
    (Variables|Default|SetVisited true)
    (Input|EnableInput (Game|GetPlayerController 0))
    (bind _asfirst_person_character_2 (Utilities|Casting|CastToFirstPersonCharacter _returnvalue))
    (Default|Cablesound _asfirst_person_character_2)))

(event OnComponentEndOverlap(CableRange)
  (params (OverlappedComponent :type Primitive%20Component%20Object%20Reference) (OtherActor :type Actor%20Object%20Reference) (OtherComp :type Primitive%20Component%20Object%20Reference) (OtherBodyIndex :type Integer))
  (bind _cuff (Variables|Default|GetCuff))
  ;[1 1 1] Release Cuff
  (Utilities|Casting|CastToCapsuleComponent OtherComp)
  (Rendering|SetVisibility _cuff false false)
  (Class|CableComponent|SetAttachEndto _cuff 0 "None" "None")
  (Input|DisableInput (Game|GetPlayerController 0)))

(event Custom|UpdateCableMats
  ;[1 1 1] Updating Cable Material
  (bind _asfirst_person_character (Utilities|Casting|CastToFirstPersonCharacter (Game|GetPlayerCharacter 0)))
  (bind _returnvalue (Class|MindtheChainCharacter|GetPower (Variables|Default|GetPcharacter)))
  (if (== (Math|Float|Round _returnvalue) 4)
    (Default|ParticleVisibleon _asfirst_person_character)
    (Default|Toolsoundon _asfirst_person_character)
    (else
      (Default|ParticleVisibleOff _asfirst_person_character)
      (Default|Toolsoundoff _asfirst_person_character)))
  (switch int (Math|Float|Round _returnvalue)
    (:1
      (CallFunction|SetCableMat "0.147962,0.791667,0.768036" "0.147962,0.791667,0.768036")
      (Default|SetCableMaterial _asfirst_person_character "0.147962,0.791667,0.768036" "0.147962,0.791667,0.768036"))
    (:2
      (CallFunction|SetCableMat "0.173884,0.791667,0.000000" "0.147962,0.791667,0.768036")
      (Default|SetCableMaterial _asfirst_person_character "0.173884,0.791667,0.000000" "0.173884,0.791667,0.000000"))
    (:3
      (CallFunction|SetCableMat "0.791667,0.776031, 0" "0.173884,0.791667, 0")
      (Default|SetCableMaterial _asfirst_person_character "0.791667,0.776031, 0" "0.791667,0.776031, 0"))
    (:4
      (CallFunction|SetCableMat "0.791667,0.000000,0.045761" "0.791667,0.776031, 0")
      (Default|SetCableMaterial _asfirst_person_character "0.791667,0.000000,0.045761" "0.791667,0.000000,0.045761"))))

(event Input|MouseEvents|LeftMouseButton
  (params (Key :type Key%20Structure))
  (bind _pcharacter (Variables|Default|GetPcharacter))
  (bind _portal_range (Variables|Default|GetPortal%20Range))
  (bind _pcharacter_2 (Variables|Default|GetPcharacter))
  (bind _pcharacter_3 (Variables|Default|GetPcharacter))
  (bind _pcharacter_4 (Variables|Default|GetPcharacter))
  (bind _returnvalue (Physics|GetCenterOfMass _portal_range "None"))
  ;[1 1 1] Set Portal
  (:Pressed
    (bind _isitactive (CallFunction|Getportalgun))
    (if _isitactive
      (bind _returnvalue_2 (Class|MindtheChainCharacter|GetTransit _pcharacter))
      (if (not _returnvalue_2)
        (if (Variables|Default|GetPortalActive)
          (bind _returnvalue_3 (Class|MindtheChainCharacter|GetRecentlyPorted _pcharacter_2))
          (if (and (not _returnvalue_3) (Variables|Default|GetPortalActive))
            (bind _returnvalue_4 (Class|MindtheChainCharacter|GetPortalCoordinates _pcharacter_2 _returnvalue))
            (if (not (Math|Vector|Equal(Vector) _returnvalue_4 "0, 0, 0" 0.0001))
              (Class|MindtheChainCharacter|SetRecentlyPorted _pcharacter_2 true)
              (bind _returnvalue_5 (Class|MindtheChainCharacter|GetVol _pcharacter_2))
              (Audio|PlaySoundatLocation "/Game/Audio/482231__veromarengere__02-lasers.482231__veromarengere__02-lasers" _returnvalue "0, 0, 0" (* _returnvalue_5 1.0) 1.0 0.0 "/Game/Audio/NewSoundAttenuation.NewSoundAttenuation" 0 0)
              (Transformation|Teleport (Game|GetPlayerCharacter 0) _returnvalue_4 "0, 0, 0")
              ;[1 1 1] Hack -> Component your teleporting to begins its overlap function before this fires
              (Class|MindtheChainCharacter|SetRecentlyPorted _pcharacter_2 false)
              (Class|MindtheChainCharacter|GetPortalLocationDefinition (Variables|Default|GetPcharacter) "0, 0, 0")
              (Class|MindtheChainCharacter|SetTransit _pcharacter_3 true)
              (Utilities|FlowControl|Delay 3.0)
              (Class|MindtheChainCharacter|SetTransit _pcharacter_3 false)
              (Physics|SetSimulatePhysics (Variables|/Script/Engine.StaticMeshActor|GetStaticMeshComponent (stale OnComponentBeginOverlap(PortalRange) _asmod_block)) false)
              (Physics|SetEnableGravity (Variables|/Script/Engine.StaticMeshActor|GetStaticMeshComponent (stale OnComponentBeginOverlap(PortalRange) _asmod_block)) false)))
          (else
            (bind _returnvalue_6 (Class|MindtheChainCharacter|GetPower _pcharacter))
            (if (and (>= _returnvalue_6 4.0) (not (Variables|Default|GetWellActive)))
              (Class|MindtheChainCharacter|SetPortalDictionary _pcharacter _returnvalue)
              (Rendering|SetVisibility (Variables|Default|GetPortal) true false)
              (Rendering|SetVisibility (Variables|Default|GetSpotLight) true false)
              (Variables|Default|SetPortalActive true)
              (Class|MindtheChainCharacter|RemovePower _pcharacter_4)
              (CallFunction|UpdateCableMats)
              (bind _asfirst_person_character (Utilities|Casting|CastToFirstPersonCharacter _pcharacter_4))
              (Variables|/Game/FirstPersonCPP/Blueprints/FirstPersonCharacter.FirstPersonCharacter_C|Setrecentlyactivated _asfirst_person_character true)
              (bind _returnvalue_7 (Class|MindtheChainCharacter|GetVol _pcharacter_4))
              (Audio|PlaySoundatLocation "/Game/Audio/494687__phonosupf__violin-static_Cue.494687__phonosupf__violin-static_Cue" _returnvalue "0, 0, 0" (* _returnvalue_7 0.5) 1.0 0.0 "/Game/Audio/NewSoundAttenuation.NewSoundAttenuation" 0 0)
              (bind _growrate (Timeline|growportal Play)
                (:Update
                  (Transformation|SetWorldScale3D (Variables|Default|GetPortal) (Math|Vector|MakeVector _growrate _growrate 1.0)))))))))))

(event Input|MouseEvents|RightMouseButton
  (params (Key :type Key%20Structure))
  (bind _pcharacter (Variables|Default|GetPcharacter))
  (bind _pcharacter_2 (Variables|Default|GetPcharacter))
  (bind _pcharacter_3 (Variables|Default|GetPcharacter))
  (bind _cuberoot (Variables|Default|GetCubeRoot))
  (bind _portal_range (Variables|Default|GetPortal%20Range))
  (bind _returnvalue (Physics|GetCenterOfMass _portal_range "None"))
  (bind _returnvalue_2 (Transformation|GetActorRotation _cuberoot))
  ;[1 1 1] Set Well
  (:Pressed
    (bind _isitactive (CallFunction|Getgravitygun))
    (if _isitactive
      (bind _returnvalue_3 (Class|MindtheChainCharacter|GetTransit (Variables|Default|GetPcharacter)))
      (if (not _returnvalue_3)
        (if (Variables|Default|GetWellActive)
          (bind _returnvalue_4 (Class|MindtheChainCharacter|GetFlipped (Variables|Default|GetPcharacter)))
          (Development|PrintString (Utilities|String|ToString(Boolean) _returnvalue_4) false)
          (if _returnvalue_4
            (Variables|Default|SetCurrent%20Rotation (* -1.0 (.roll _returnvalue_2)))
            (bind _gravity_rotation (Timeline|world%20rot PlayFromStart)
              (:Update
                (Transformation|SetWorldRotation (Variables|/Script/Engine.Actor|GetRootComponent (Variables|Default|GetCubeRoot)) (Math|Rotator|MakeRotator (+ _gravity_rotation (Variables|Default|GetCurrent%20Rotation)) 0.0 0.0) false false)
                (Transformation|Teleport (Game|GetPlayerCharacter 0) _returnvalue "0, 0, 0"))
              (:Finished
                (bind _returnvalue_5 (Class|MindtheChainCharacter|GetFlipped _pcharacter_2))
                (if _returnvalue_5
                  (Class|MindtheChainCharacter|SetFlipped _pcharacter_2 false)
                  (else
                    (Class|MindtheChainCharacter|SetFlipped _pcharacter_2 true)))
                (Class|MindtheChainCharacter|SetTransit _pcharacter_3 true)
                (Utilities|FlowControl|Delay 3.0)
                (Class|MindtheChainCharacter|SetTransit _pcharacter_3 false)))
            (else
              (Variables|Default|SetCurrent%20Rotation (.roll _returnvalue_2))
              (Timeline|world%20rot PlayFromStart)))
          (else
            (bind _returnvalue_6 (Class|MindtheChainCharacter|GetPower (Variables|Default|GetPcharacter)))
            (if (and (>= _returnvalue_6 4.0) (not (Variables|Default|GetPortalActive)))
              (Rendering|SetVisibility (Variables|Default|GetGravityWell) true false)
              (Rendering|SetVisibility (Variables|Default|Getgravparticles) true false)
              (Variables|Default|SetWellActive true)
              (Class|MindtheChainCharacter|RemovePower _pcharacter)
              (CallFunction|UpdateCableMats)
              (bind _asfirst_person_character (Utilities|Casting|CastToFirstPersonCharacter _pcharacter))
              (Variables|/Game/FirstPersonCPP/Blueprints/FirstPersonCharacter.FirstPersonCharacter_C|Setrecentlyactivated _asfirst_person_character true)
              (bind _returnvalue_7 (Class|MindtheChainCharacter|GetVol _pcharacter))
              (Audio|PlaySoundatLocation "/Game/Audio/470903__samsterbirdies__laser_Cue.470903__samsterbirdies__laser_Cue" _returnvalue "0, 0, 0" (* _returnvalue_7 0.5) 1.0 0.0 "/Game/Audio/NewSoundAttenuation.NewSoundAttenuation" 0 0))))))))

(fn ConstructionScript
  (Rendering|Material|CreateDynamicMaterialInstance (Variables|Default|GetGrid) 0 0 "None" :!class /Script/Engine.PrimitiveComponent)
  (Rendering|Material|CreateDynamicMaterialInstance (Variables|Default|GetCuff) 0 0 "None" :!class /Script/Engine.PrimitiveComponent))

(fn SetCableMat
  (params (CuffVector :type Vector) (GridVector :type Vector))
  (Rendering|Material|SetVectorParameterValueonMaterials (Variables|Default|GetCuff) "CableColor" CuffVector)
  (Rendering|Material|SetVectorParameterValueonMaterials (Variables|Default|GetGrid) "CableColor" GridVector))

(fn Getportalgun
  (bind _asfirst_person_character (Utilities|Casting|CastToFirstPersonCharacter (Variables|Default|GetPcharacter)))
  (return (Variables|/Game/FirstPersonCPP/Blueprints/FirstPersonCharacter.FirstPersonCharacter_C|Getportalgunactive _asfirst_person_character)))

(fn Getgravitygun
  (bind _asfirst_person_character (Utilities|Casting|CastToFirstPersonCharacter (Variables|Default|GetPcharacter)))
  (return (Variables|/Game/FirstPersonCPP/Blueprints/FirstPersonCharacter.FirstPersonCharacter_C|Getgravitygunactive _asfirst_person_character)))