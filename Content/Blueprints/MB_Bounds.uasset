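; MB_Bounds is a trigger volume that locks any Mod_Block entering its Box into place on a referenced Lock.
; On overlap it plays a spatialized sound at the block's mesh, with volume taken from the player's MindTheChainCharacter.
; It then turns off physics simulation on that mesh and attaches it to the Lock's root component, keeping its world transform.
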(event OnComponentBeginOverlap(Box)
  (params (OverlappedComponent :type Primitive%20Component%20Object%20Reference) (OtherActor :type Actor%20Object%20Reference) (OtherComp :type Primitive%20Component%20Object%20Reference) (OtherBodyIndex :type Integer) (bFromSweep :type Boolean) (SweepResult :type Hit%20Result%20Structure%20%28by%20ref%29))
  (bind _asmod_block (Utilities|Casting|CastToMod_Block OtherActor))
  (bind _asmind_the_chain_character (Utilities|Casting|CastToMindTheChainCharacter (Game|GetPlayerCharacter 0)))
  (bind _returnvalue (Class|MindtheChainCharacter|GetVol _asmind_the_chain_character))
  (Audio|PlaySoundatLocation "/Game/Audio/13946__adcbicycle__18.13946__adcbicycle__18" (Transformation|GetWorldLocation (Variables|/Script/Engine.StaticMeshActor|GetStaticMeshComponent _asmod_block)) "0, 0, 0" (* _returnvalue 1.0) 1.0 0.0 "/Game/Audio/NewSoundAttenuation.NewSoundAttenuation" 0 0)
  (Physics|SetSimulatePhysics (Variables|/Script/Engine.StaticMeshActor|GetStaticMeshComponent _asmod_block) false)
  (Transformation|AttachComponentToComponent (Variables|/Script/Engine.StaticMeshActor|GetStaticMeshComponent _asmod_block) (Variables|/Script/Engine.Actor|GetRootComponent (Variables|Default|GetLock)) "None" "KeepWorld" "KeepWorld" "KeepWorld" true))

(fn ConstructionScript)